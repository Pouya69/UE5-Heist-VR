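; Hologram effect actor for the main character that feeds the transform of its SubtractiveCollision component to materials through the MPC_Hologram parameter collection.
; UpdateCustom writes the component's world location, scale (as Bounds) and forward, right and up axes as vector parameters, describing an oriented volume.
; It runs from the Construction Script and every Tick, with a note that Tick must be enabled in Sequencer.
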(event `self.ReceiveTick`
  (params (DeltaSeconds :type "Float (single-precision)"))
  ;[1 1 1] Need to enable Tick in Sequencer
  (`self.Update_Custom`))

(fn `Update_Custom`
  (bind _subtractive_collision (`self.Subtractive_Collision`))
  (`KismetMaterialLibrary.SetVectorParameterValue` "/Game/Autoviscera/Assets/Characters/MainCharacter/Hologram/MPC_Hologram.MPC_Hologram" "Location" (`KismetMathLibrary.Conv_VectorToLinearColor` (`SceneComponent.K2_GetComponentLocation` _subtractive_collision)))
  (`KismetMaterialLibrary.SetVectorParameterValue` "/Game/Autoviscera/Assets/Characters/MainCharacter/Hologram/MPC_Hologram.MPC_Hologram" "Bounds" (`KismetMathLibrary.Conv_VectorToLinearColor` (`SceneComponent.K2_GetComponentScale` _subtractive_collision)))
  (`|ExecutionSequence`
    (:`then_0`
      (`KismetMaterialLibrary.SetVectorParameterValue` "/Game/Autoviscera/Assets/Characters/MainCharacter/Hologram/MPC_Hologram.MPC_Hologram" "X" (`KismetMathLibrary.Conv_VectorToLinearColor` (`SceneComponent.GetForwardVector` _subtractive_collision))))
    (:`then_1`
      (`KismetMaterialLibrary.SetVectorParameterValue` "/Game/Autoviscera/Assets/Characters/MainCharacter/Hologram/MPC_Hologram.MPC_Hologram" "Y" (`KismetMathLibrary.Conv_VectorToLinearColor` (`SceneComponent.GetRightVector` _subtractive_collision))))
    (:`then_2`
      (`KismetMaterialLibrary.SetVectorParameterValue` "/Game/Autoviscera/Assets/Characters/MainCharacter/Hologram/MPC_Hologram.MPC_Hologram" "Z" (`KismetMathLibrary.Conv_VectorToLinearColor` (`SceneComponent.GetUpVector` _subtractive_collision))))))

(fn `UserConstructionScript`
  (`self.Update_Custom`))