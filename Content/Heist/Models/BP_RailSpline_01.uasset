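; Rail spline construction actor that lays a chosen mesh along a spline, either spaced or as a continuous run.
; The construction script measures the mesh along its forward axis to set section length and count.
; Spaced mode adds rotated instances to an instanced mesh component, plus spline mesh components left without a mesh.
; Continuous mode bends collisionless spline meshes between sampled points, with tangents clamped to mesh length.
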(fn `Get Location and Tangent`
  (params (Index :type Integer))
  (returns (Location :type "Vector Structure") (Tangent :type "Vector Structure"))
  (bind _spline1 (`self.Spline1`))
  (bind _returnvalue (* Index (`self.Mesh Length`)))
  (return (`SplineComponent.GetLocationAtDistanceAlongSpline` _spline1 _returnvalue "Local") (`KismetMathLibrary.ClampVectorSize` (`SplineComponent.GetTangentAtDistanceAlongSpline` _spline1 _returnvalue "Local") 0.0 (`self.Mesh Length`))))

(fn `UserConstructionScript`
  (locals (Index :type Integer) (`Spline Mesh Instanced` :type "StaticMesh Object Reference") (ISM :type "InstancedStaticMeshComponent Object Reference"))
  (bind _forward_axis (`self.Forward Axis`))
  (bind _index (`local.Index`))
  (bind _spline1 (`self.Spline1`))
  (bind (_returnvalue_min _returnvalue_max) (break `Box` (`StaticMesh.GetBoundingBox` (`local.Spline Mesh Instanced`))))
  (bind (_location _tangent) (`self.Get Location and Tangent` _index))
  (bind _returnvalue (* (`self.Mesh Length`) (`local.Index`)))
  (bind _returnvalue_2 (* (`self.Mesh Length`) (`local.Index`)))
  (bind _returnvalue_3 (* (`self.Section Length`) (`local.Index`)))
  (bind (_location_2 _tangent_2) (`self.Get Location and Tangent` (+ _index 1)))
  (bind (_returnvalue_x _returnvalue_y _returnvalue_z) (`KismetMathLibrary.BreakVector` (- _returnvalue_max _returnvalue_min)))
  (bind _returnvalue_4 (+ _returnvalue (`self.Mesh Length`)))
  (bind _returnvalue_5 (+ _returnvalue_2 (`self.Mesh Length`)))
  (bind _returnvalue_6 (`KismetMathLibrary.SelectFloat` _returnvalue_2 _returnvalue_5 (< _returnvalue_2 _returnvalue_5)))
  (bind _returnvalue_7 (`KismetMathLibrary.SelectFloat` _returnvalue _returnvalue_4 (< _returnvalue _returnvalue_4)))
  (bind _returnvalue_8 (`KismetMathLibrary.MakeTransform` (`SplineComponent.GetLocationAtDistanceAlongSpline` _spline1 _returnvalue_3 "Local") (`KismetMathLibrary.ComposeRotators` (`self.Mesh Rotation`) (`SplineComponent.GetRotationAtDistanceAlongSpline` _spline1 _returnvalue_3 "Local"))))
  (`|ExecutionSequence`
    (:`then_0`
      (bind _returnvalue_9 (`AddComponent|NODE_AddInstancedStaticMeshComponent-1`))
      (`StaticMeshComponent.SetStaticMesh` _returnvalue_9 (`self.Spline Meshs`))
      (set `local.Spline Mesh Instanced` (`StaticMeshComponent.StaticMesh` _returnvalue_9))
      (set `local.ISM` _returnvalue_9))
    (:`then_1`
      (if (`|EnumEquality` _forward_axis "X")
        (set `self.Mesh Length` _returnvalue_x)
        (elif (`|EnumEquality` _forward_axis "Y")
          (set `self.Mesh Length` _returnvalue_y)
          (else
            (set `self.Mesh Length` _returnvalue_z))))
      (if (`self.Space Meshes`)
        (set `self.Section Length` (+ (`self.Mesh Length`) (`self.Spacing`)))
        (for _index_2 (range (+ (/ (`SplineComponent.GetSplineLength` _spline1) (`KismetMathLibrary.FTrunc` (`self.Section Length`))) 1))
          (set `local.Index` _index_2)
          (bind _returnvalue_10 (`AddComponent|NODE_AddSplineMeshComponent-0` :`RelativeTransform` _returnvalue_8))
          (`InstancedStaticMeshComponent.AddInstance` (`local.ISM`) _returnvalue_8 false)
          (`PrimitiveComponent.SetCollisionEnabled` _returnvalue_10 "NoCollision")
          (`SplineMeshComponent.SetForwardAxis` _returnvalue_10 (`self.Forward Axis`) true)
          (`SplineMeshComponent.SetSplineUpDir` _returnvalue_10 (`SplineComponent.GetUpVectorAtDistanceAlongSpline` (`self.Spline1`) (+ (/ (- _returnvalue_7 _returnvalue) 2.0) _returnvalue_7) "Local") true))
        (else
          (for _index_3 (range (+ (/ (`SplineComponent.GetSplineLength` (`self.Spline1`)) (`KismetMathLibrary.FTrunc` (`self.Mesh Length`))) 1))
            (set `local.Index` _index_3)
            (bind _returnvalue_11 (`AddComponent|NODE_AddSplineMeshComponent-1`))
            (`StaticMeshComponent.SetStaticMesh` _returnvalue_11 (`local.Spline Mesh Instanced`))
            (`PrimitiveComponent.SetCollisionEnabled` _returnvalue_11 "NoCollision")
            (`SplineMeshComponent.SetForwardAxis` _returnvalue_11 (`self.Forward Axis`) true)
            (`SplineMeshComponent.SetStartAndEnd` _returnvalue_11 _location _tangent _location_2 _tangent_2 true)
            (`SplineMeshComponent.SetSplineUpDir` _returnvalue_11 (`SplineComponent.GetUpVectorAtDistanceAlongSpline` (`self.Spline1`) (+ (/ (- _returnvalue_6 _returnvalue_2) 2.0) _returnvalue_6) "Local") true)))))))