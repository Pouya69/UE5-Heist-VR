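; Courier character Blueprint for the Heist credits sequence, handling player size changes, slow motion and cutscene interrupts.
; A size-change handler rescales movement speed, acceleration, step height and mass for TINY or MEDIUM, though its game mode binding never runs.
; Slow-down halves credits audio pitch and pushes a sound mix, then a timer restores both.
; TESTONLY functions start cutscenes or test time dilation.
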(event `self.ReceiveBeginPlay`
  (set `self.bIsInDefaultCutsceneActions` false))

(event `OnPlayerChangeSize_Event`
  (params (NewPlayerSize :type "EHeistSize Enum" :default "TINY"))
  (bind _returnvalue (select `EHeistSize` NewPlayerSize :`TINY` 1000.0 :`MEDIUM` 1.0 :!type "Float (single-precision)"))
  (bind _charactermovement (`self.CharacterMovement`))
  (set `self.CurrentSize` NewPlayerSize)
  (`CharacterMovementComponent.SetMovementMode` _charactermovement "MOVE_None" 0)
  (`KismetSystemLibrary.DelayUntilNextTick`)
  (set `CharacterMovementComponent.MaxAcceleration` (* _returnvalue 2048.0) _charactermovement)
  (set `CharacterMovementComponent.MaxWalkSpeed` (* (`self.BaseMovementSpeed`) _returnvalue) _charactermovement)
  (set `CharacterMovementComponent.MaxStepHeight` (* _returnvalue 45.0) _charactermovement)
  (set `CharacterMovementComponent.Mass` (* _returnvalue 100.0) _charactermovement)
  (set `MovementComponent.Velocity` (0.0 0.0 0.0) _charactermovement)
  (`CharacterMovementComponent.SetMovementMode` _charactermovement "MOVE_Walking" 0))

(event `self.InterruptedCutscene`
  (params (bEndCurrentCutscene :type Boolean))
  (`parent.InterruptedCutscene` bEndCurrentCutscene))

(event `self.ReceiveTick`
  (params (DeltaSeconds :type "Float (single-precision)")))

(event `HeistInteractionInterface.ObjectOutOfSlowMotion`
  (`AudioComponent.SetPitchMultiplier` (`AmbientSound.AudioComponent` (`self.Credits Sound Ref`)) 1.0)
  (set `self.CustomTimeDilation` 1.0)
  (`parent.ObjectOutOfSlowMotion`)
  (`GameplayStatics.ClearSoundMixModifiers`))

(event `HeistInteractionInterface.ObjectSlowedDown`
  (`parent.ObjectSlowedDown`)
  (`AudioComponent.SetPitchMultiplier` (`AmbientSound.AudioComponent` (`self.Credits Sound Ref`)) 0.5)
  (`KismetSystemLibrary.K2_ClearAndInvalidateTimerHandle` (`self.Custom Timer Dilation`))
  (`GameplayStatics.PushSoundMixModifier` "/Game/Audio_P1/System/SM_SlowMotion.SM_SlowMotion")
  (bind _returnvalue (`KismetSystemLibrary.K2_SetTimerDelegate` (delegate `HeistInteractionInterface.ObjectOutOfSlowMotion`) 2.5))
  (set `self.Custom Timer Dilation` _returnvalue))

(fn `TESTONLY_SETDEFAULTFALSE`
  (set `self.bIsInDefaultCutsceneActions` false))

(fn `TESTONLY_StartFirstCutscene`
  (`MovieSceneSequencePlayer.Play` (`LevelSequenceActor.SequencePlayer` (`self.FirstCutsceneRef`))))

(fn `TESTONLY_StartLedgeCutscene`
  (set `self.bIsInDefaultCutsceneActions` false)
  (`MovieSceneSequencePlayer.Play` (`LevelSequenceActor.SequencePlayer` (`self.LedgeCutsceneRef`))))

(fn `TESTONLY_StartPistolCutscene`
  (`MovieSceneSequencePlayer.Play` (`LevelSequenceActor.SequencePlayer` (`self.PistolCutsceneRef`))))

(fn `TESTONLY_StartRustyValveCutscene`
  (set `self.bIsInDefaultCutsceneActions` false)
  (`MovieSceneSequencePlayer.Play` (`LevelSequenceActor.SequencePlayer` (`self.RustyValveCutsceneRef`))))

(fn `TESTONLY_TimeDilation`
  (`HeistFunctionLibrary.SetTimeDilationOfObject` self 0.1 8.0))

(fn `UserConstructionScript`)