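; Elevator lever for the Heist environment that extends its parent's interaction with an indicator light.
; At BeginPlay it creates a dynamic material for the Plane mesh and enables the lever.
; Interacting runs the parent logic and turns the light green, while returning to the starting point sends a reset message to the linked actor and turns it red.
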(event `self.ReceiveBeginPlay`
  (bind _plane (`self.Plane`))
  (bind _returnvalue (`PrimitiveComponent.CreateDynamicMaterialInstance` _plane 0 (`PrimitiveComponent.GetMaterial` _plane 0) "None"))
  (bind _output_get (set `self.MID_LeverLight` _returnvalue))
  (`PrimitiveComponent.SetMaterial` _plane 0 _output_get)
  (`self.ToggleLeverEnabled` true))

(event `self.LeverAtStartingPoint`
  (message `HeistInteractionInterface.Interact_Reset` (`self.LinkedActor`))
  (`self.LeverLightStatus` false))

(event `HeistInteractionInterface.Interact`
  (`parent.Interact`)
  (`self.LeverLightStatus` true))

(event `self.LeverLightStatus`
  (params (bIsActive :type Boolean))
  (bind _mid_leverlight (`self.MID_LeverLight`))
  (`|ExecutionSequence`
    (:`then_0`
      (`MaterialInstanceDynamic.SetVectorParameterValue` _mid_leverlight "Color_Emissive" (`KismetMathLibrary.SelectColor` (struct :`G` 1.0 :`A` 1.0) (struct :`R` 1.0 :`A` 1.0) bIsActive)))
    (:`then_1`
      (`MaterialInstanceDynamic.SetScalarParameterValue` _mid_leverlight "EMissive\\" 20.0))))

(fn `UserConstructionScript`)