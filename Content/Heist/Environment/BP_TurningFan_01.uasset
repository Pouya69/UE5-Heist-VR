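; Spinning fan obstacle in Heist that players can pass through while it is slowed down.
; Game mode size changes show and spin it when sizes match, otherwise hide, silence, rescale and reposition it.
; Slow motion cuts time dilation and sound pitch and turns the collision box into a player trigger.
; Leaving slow motion restores pitch and blocking, first teleporting one overlapping pawn outward along the box's local Y axis.
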(event `self.ReceiveBeginPlay`
  (`AudioComponent.Play` (`AmbientSound.AudioComponent` (`self.Fan Sound Ref`)) 0.0)
  (set `self.Initial Size` (`self.GetActorScale3D`))
  (set `self.Initial_Location` (`self.K2_GetActorLocation`))
  (bind _asheist_game_mode (cast `HeistGameMode` (`GameplayStatics.GetGameMode`)))
  (add `HeistGameMode.OnPlayerChangeSize` _asheist_game_mode (delegate `OnPlayerChangeSize_Event`))
  (`self.OnPlayerChangeSize_Event` "MEDIUM"))

(event `OnPlayerChangeSize_Event`
  (params (NewPlayerSize :type "EHeistSize Enum" :default "TINY"))
  (bind _fanbase (`self.FanBase`))
  (bind _audiocomponent (`AmbientSound.AudioComponent` (`self.Fan Sound Ref`)))
  (if (`|EnumEquality` NewPlayerSize (`self.Current Size`))
    (`self.SetActorTickEnabled` true)
    (`SceneComponent.SetVisibility` _fanbase true true)
    (message `AudioParameterControllerInterface.SetBoolParameter` _audiocomponent "Fan_Play" true)
    (bind (_direction _prepellar_rotation) (`Timeline|Prepellar Timeline` :!label _label)
      (:`Update`
        (`SceneComponent.K2_SetRelativeRotation` (`self.Prepellar`) (`KismetMathLibrary.MakeRotator` 0.0 -90.0 _prepellar_rotation) false false)))
    (else
      (`self.SetActorTickEnabled` false)
      (`SceneComponent.SetVisibility` _fanbase false true)
      (message `AudioParameterControllerInterface.SetBoolParameter` _audiocomponent "Fan_Stop" true)
      (`self.SetActorScale3D` (* (`self.Initial Size`) (select `EHeistSize` NewPlayerSize :`TINY` 1000.0 :`MEDIUM` 1.0)))
      (`self.K2_SetActorLocation` (* (`self.Initial_Location`) (select `EHeistSize` NewPlayerSize :`TINY` 1000.0 :`MEDIUM` 1.0)) false true)
      (goto _label :!via `Stop`))))

(event `HeistInteractionInterface.ObjectSlowedDown`
  (set `self.CustomTimeDilation` (/ (`self.CustomTimeDilation`) 6.0))
  (`PrimitiveComponent.SetCollisionProfileName` (`self.BoxColl`) "Player_Trigger_Only" true)
  (`AudioComponent.SetPitchMultiplier` (`AmbientSound.AudioComponent` (`self.Fan Sound Ref`)) 0.5))

(event `HeistInteractionInterface.ObjectOutOfSlowMotion`
  (bind _returnvalue (`SceneComponent.K2_GetComponentToWorld` (`self.BoxColl`)))
  (`AudioComponent.SetPitchMultiplier` (`AmbientSound.AudioComponent` (`self.Fan Sound Ref`)) 1.0)
  (for _array_element (`PrimitiveComponent.GetOverlappingActors` (`self.BoxColl`) "/Script/Engine.Pawn")
    (bind (_returnvalue_location _returnvalue_rotation _returnvalue_scale) (`KismetMathLibrary.BreakTransform` (`self.GetTransform` _array_element)))
    (bind _returnvalue_2 (`KismetMathLibrary.MakeRelativeTransform` (`KismetMathLibrary.MakeTransform` _returnvalue_location _returnvalue_rotation _returnvalue_scale) _returnvalue))
    (`self.K2_SetActorLocation` _array_element (`KismetMathLibrary.TransformLocation` _returnvalue (`KismetMathLibrary.MakeVector` (.x (.location _returnvalue_2)) (* (.y (.location _returnvalue_2)) 4.0) (.z (.location _returnvalue_2)))) false true)
    (break))
  (`PrimitiveComponent.SetCollisionProfileName` (`self.BoxColl`) "BlockAll" true))

(event `HeistInteractionInterface.SetNewSizeTo`
  (params (NewSize :type "EHeistSize Enum" :default "TINY")))

(fn `Dilation_TEST`
  (`HeistFunctionLibrary.SetTimeDilationOfObject` self 0.1 4.0))

(fn `GetAnchorSceneComponentForWheel`
  (returns (ReturnValue :type "SceneComponent Object Reference"))
  (return null))

(fn `GetCurrentSizeOfGameObject`
  (returns (ReturnValue :type "EHeistSize Enum"))
  (return (`self.Current Size`)))

(fn `GetGrabComponents`
  (returns (OutGrabComponents :type "Array of HeistGrabComponent Object Reference") (ReturnValue :type Boolean))
  (return _ false))

(fn `GetHandAnimationType`
  (returns (ReturnValue :type "EHeistGrabHandState Enum"))
  (return "DEFAULT"))

(fn `GetIsInteractable`
  (returns (ReturnValue :type Boolean))
  (return false))

(fn `GetPhysicsConstraintComp`
  (returns (ReturnValue :type "PhysicsConstraintComponent Object Reference"))
  (return null))

(fn `IsGrabbable`
  (params (BoneHit :type Name))
  (returns (ReturnValue :type Boolean))
  (return false))

(fn `IsRemoteGrabbable`
  (returns (ReturnValue :type Boolean))
  (return false))

(fn `Play Sound Test`
  (`AudioParameterControllerInterface.SetTriggerParameter` (`AmbientSound.AudioComponent` (`self.Fan Sound Ref`)) "Fan_Play"))

(fn `RemoteGrab`
  (returns (ReturnValue :type Boolean))
  (return false))

(fn `Reset Dilation`
  (set `self.CustomTimeDilation` 1.0))

(fn `UserConstructionScript`)