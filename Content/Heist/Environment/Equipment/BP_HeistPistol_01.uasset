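; BP_HeistPistol_01 is the hand-held pistol in the Heist environment, equipped to either the left or right hand.
; Equipping notifies its owner, enables input and adds the left or right weapon mapping context; unequipping reverses this.
; The shoot action for the equipped hand notifies the owner, calls ShootPistol, drives the pistol anim instance and triggers the gun sound through an audio parameter.
; Releasing the trigger notifies the owner and anim instance.
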(event `self.ReceiveBeginPlay`)

(event `self.OnHeistPistolEquipped`
  (message `HeistPlayerInterface.PistolEquipped` (`self.GetOwner`))
  (`self.EnableInput` (`GameplayStatics.GetPlayerController` 0))
  (`EnhancedInputSubsystemInterface.AddMappingContext` (pcsubsystem `EnhancedInputLocalPlayerSubsystem` (`GameplayStatics.GetPlayerController` 0)) (select `bool` (`self.bIsRightHandEquipped`) :`false` "/Game/VRTemplate/Input/IMC_Weapon_Left.IMC_Weapon_Left" :`true` "/Game/VRTemplate/Input/IMC_Weapon_Right.IMC_Weapon_Right" :!type "InputMappingContext Object Reference") 1 (struct)))

(event `self.OnHeistPistolUnequipped`
  (message `HeistPlayerInterface.PistolUnequipped` (`self.GetOwner`))
  (`self.DisableInput` (`GameplayStatics.GetPlayerController` 0))
  (`EnhancedInputSubsystemInterface.RemoveMappingContext` (pcsubsystem `EnhancedInputLocalPlayerSubsystem` (`GameplayStatics.GetPlayerController` 0)) (select `bool` (`self.bIsRightHandEquipped`) :`false` "/Game/VRTemplate/Input/IMC_Weapon_Left.IMC_Weapon_Left" :`true` "/Game/VRTemplate/Input/IMC_Weapon_Right.IMC_Weapon_Right" :!type "InputMappingContext Object Reference") (struct)))

(event `EnhancedInput|/Game/VRTemplate/Input/Actions/IA_Shoot_Left`
  (params (ActionValue :type Boolean) (ElapsedSeconds :type "Float (double-precision)") (TriggeredSeconds :type "Float (double-precision)") (InputAction :type "InputAction Object Reference" :default "/Game/VRTemplate/Input/Actions/IA_Shoot_Left.IA_Shoot_Left"))
  (:`Triggered`
    (if (not (`self.bIsRightHandEquipped`))
      (message `HeistPlayerInterface.PistolTriggerHeldDown` (`self.GetOwner`) :!label _label)
      (`self.ShootPistol`)
      (`HeistPistolAnimInstance.PistolShot` (`self.PistolAnimInstance`))
      (`AudioParameterControllerInterface.SetBoolParameter` (`self.Shoot Sound`) "Play_TimeGun" true))))

(event `EnhancedInput|/Game/VRTemplate/Input/Actions/IA_Shoot_Right`
  (params (ActionValue :type Boolean) (ElapsedSeconds :type "Float (double-precision)") (TriggeredSeconds :type "Float (double-precision)") (InputAction :type "InputAction Object Reference" :default "/Game/VRTemplate/Input/Actions/IA_Shoot_Right.IA_Shoot_Right"))
  (:`Triggered`
    (if (`self.bIsRightHandEquipped`)
      (goto _label))))

(event `EnhancedInput|/Game/VRTemplate/Input/Actions/IA_Shoot_Left_Released`
  (params (ActionValue :type Boolean) (ElapsedSeconds :type "Float (double-precision)") (TriggeredSeconds :type "Float (double-precision)") (InputAction :type "InputAction Object Reference" :default "/Game/VRTemplate/Input/Actions/IA_Shoot_Left_Released.IA_Shoot_Left_Released"))
  (:`Triggered`
    (if (not (`self.bIsRightHandEquipped`))
      (message `HeistPlayerInterface.PistolTriggerReleased` (`self.GetOwner`) :!label _label_2)
      (`HeistPistolAnimInstance.PistolTriggerReleased` (`self.PistolAnimInstance`)))))

(event `EnhancedInput|/Game/VRTemplate/Input/Actions/IA_Shoot_Right_Released`
  (params (ActionValue :type Boolean) (ElapsedSeconds :type "Float (double-precision)") (TriggeredSeconds :type "Float (double-precision)") (InputAction :type "InputAction Object Reference" :default "/Game/VRTemplate/Input/Actions/IA_Shoot_Right_Released.IA_Shoot_Right_Released"))
  (:`Triggered`
    (if (`self.bIsRightHandEquipped`)
      (goto _label_2))))

(fn `UserConstructionScript`)