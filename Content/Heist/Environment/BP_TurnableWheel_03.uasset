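; BP_TurnableWheel_03 is an unfinished turnable wheel prop with a grab component, and it currently does nothing at runtime.
; Its grab, release and timer events are all empty.
; Disconnected nodes sketch the intended technique: a looping timer rolls the wheel mesh based on the look-at direction to the holding motion controller, dotted with the wheel's right vector.
; A disconnected timer pause is also present.
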(event `self.GrabComponent.OnGrabbed`
  (params (GrabbedComponent :type "HeistGrabComponent Object Reference") (MotionControllerRef :type "HeistMotionControllerComponent Object Reference")))

(event `WheelCustom_Event`)

(event `self.GrabComponent.OnReleased`
  (params (GrabbbedComponent :type "HeistGrabComponent Object Reference") (MotionControllerRef :type "HeistMotionControllerComponent Object Reference")))

(fn `UserConstructionScript`)