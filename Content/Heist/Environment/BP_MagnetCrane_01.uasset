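; BP_MagnetCrane_01 is a magnet crane for the Heist environment, a child Blueprint that relies on its parent for interaction.
; Construction places the IK location at a starting distance along the actor's negative right vector.
; Add and Subtract functions nudge normalized yaw and height in fixed steps through SetAmount and SetAmount02.
; Toggle Active Radial just calls Interact, which defers to the parent, leaving local radial force and focus-message nodes unconnected.
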(event `HeistInteractionInterface.Interact`
  (`parent.Interact`))

(fn `SetAmount1_Add`
  (`HeistInteractionInterface.SetAmount` (+ (`self.CurrentYawNormalized`) 0.1)))

(fn `SetAmount1_Subtract`
  (`HeistInteractionInterface.SetAmount` (+ (`self.CurrentYawNormalized`) -0.1)))

(fn `SetAmount2_Add`
  (`HeistInteractionInterface.SetAmount_02` (+ (`self.CurrentHeightNormalized`) 0.1)))

(fn `SetAmount2_Subtract`
  (`HeistInteractionInterface.SetAmount_02` (+ (`self.CurrentHeightNormalized`) -0.1)))

(fn `Toggle Active Radial`
  (`HeistInteractionInterface.Interact`))

(fn `UserConstructionScript`
  (set `self.IK_Location` (+ (`self.K2_GetActorLocation`) (* (`KismetMathLibrary.NegateVector` (`self.GetActorRightVector`)) (`self.StartingDistance`)))))