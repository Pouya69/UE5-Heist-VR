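; BP_TinyLever_01 is a small grabbable, interactable lever environment prop for Heist that resets a linked actor.
; Interact defers to the parent implementation, and returning to the starting point sends an interact reset message to LinkedActor.
; Its grab and interact queries always return true and expose GrabComponent as the only grab target.
; A call to disable the lever is left unconnected and never runs.
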(event `self.ReceiveBeginPlay`)

(event `self.LeverAtStartingPoint`
  (message `HeistInteractionInterface.Interact_Reset` (`self.LinkedActor`)))

(event `HeistInteractionInterface.Interact`
  (`parent.Interact`))

(fn `GetGrabComponents`
  (returns (OutGrabComponents :type "Array of HeistGrabComponent Object Reference") (ReturnValue :type Boolean))
  (return (`|MakeArray` (`self.GrabComponent`)) true))

(fn `GetIsInteractable`
  (returns (ReturnValue :type Boolean))
  (return true))

(fn `IsGrabbable`
  (params (BoneHit :type Name))
  (returns (ReturnValue :type Boolean))
  (return true))

(fn `UserConstructionScript`)