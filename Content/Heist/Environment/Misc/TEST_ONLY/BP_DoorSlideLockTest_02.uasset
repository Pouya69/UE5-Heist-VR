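; Test VR sliding door-lock actor, built as a grabbable Heist interactable with a single Cube mesh.
; On BeginPlay it initializes two grab components on the Cube and disables physics simulation on drop, then exposes both through the grab interface.
; It reports itself as grabbable, tiny and not remote-grabbable.
; Disconnected leftover logic would constrain the physics hand to the Cube's local X axis; the custom tick is empty.
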(event `self.ReceiveBeginPlay`
  (bind _heistgrabcomp (`self.HeistGrabComp`))
  (bind _heistgrabcomp1 (`self.HeistGrabComp1`))
  (`HeistGrabComponent.InitializeGrabComponent` _heistgrabcomp (`self.Cube`) true)
  (`HeistGrabComponent.SetSimulateOnDrop` _heistgrabcomp false)
  (`HeistGrabComponent.InitializeGrabComponent` _heistgrabcomp1 (`self.Cube`) true)
  (`HeistGrabComponent.SetSimulateOnDrop` _heistgrabcomp1 false))

(event `HeistInteractionInterface.Custom_Tick`
  (params (DeltaTime :type "Float (single-precision) (by ref)") (WhichGrabComponent :type "HeistGrabComponent Object Reference")))

(fn `GetAnchorSceneComponentForWheel`
  (returns (ReturnValue :type "SceneComponent Object Reference"))
  (return null))

(fn `GetCurrentSizeOfGameObject`
  (returns (ReturnValue :type "EHeistSize Enum"))
  (return "TINY"))

(fn `GetGrabComponents`
  (returns (OutGrabComponents :type "Array of HeistGrabComponent Object Reference") (ReturnValue :type Boolean))
  (return (`|MakeArray` (`self.HeistGrabComp`) (`self.HeistGrabComp1`)) true))

(fn `GetHandAnimationType`
  (returns (ReturnValue :type "EHeistGrabHandState Enum"))
  (return "DEFAULT"))

(fn `GetIsInteractable`
  (returns (ReturnValue :type Boolean))
  (return false))

(fn `IsGrabbable`
  (params (BoneHit :type Name))
  (returns (ReturnValue :type Boolean))
  (return true))

(fn `IsRemoteGrabbable`
  (returns (ReturnValue :type Boolean))
  (return false))

(fn `RemoteGrab`
  (returns (ReturnValue :type Boolean))
  (return false))

(fn `UserConstructionScript`)