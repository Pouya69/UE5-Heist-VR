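; Elevator call-down button for the Heist environment, kept in a test-only folder, that messages a linked actor and shows its state through emissive glow.
; BeginPlay shares one dynamic material between button and wires, and caches the linked actor's light root, if any.
; Focus events set the powered state and glow, messaging the linked actor when lost.
; While powered, interacting darkens it and sends a reset message, and returning to start relights it.
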(event `self.ReceiveBeginPlay`
  (bind _buttonmovingmeshcomponent (`self.ButtonMovingMeshComponent`))
  (bind _returnvalue (`PrimitiveComponent.CreateDynamicMaterialInstance` _buttonmovingmeshcomponent 0 (`PrimitiveComponent.GetMaterial` _buttonmovingmeshcomponent 0) "None"))
  (bind _output_get (set `self.Button_MID` _returnvalue))
  (for _array_element (`self.Wires`)
    (`PrimitiveComponent.SetMaterial` (`StaticMeshActor.StaticMeshComponent` _array_element) 0 _output_get))
  (`PrimitiveComponent.SetMaterial` _buttonmovingmeshcomponent 0 _output_get)
  (bind _linkedactor (`self.LinkedActor`)
    (:`then`
      (bind _aslight_component (cast `LightComponent` (`Actor.RootComponent` _linkedactor)))
      (set `self.Light_LinkedActor` _aslight_component))
    (:`else`)))

(event `HeistInteractionInterface.Interact`
  (if (`self.bIsPowered`)
    (`MaterialInstanceDynamic.SetScalarParameterValue` (`self.Button_MID`) "EMissive\\" 0.0)
    (message `HeistInteractionInterface.Interact_Reset` (`self.LinkedActor`))))

(event `self.ButtonAtStartingPoint`
  (if (`self.bIsPowered`)
    (`MaterialInstanceDynamic.SetScalarParameterValue` (`self.Button_MID`) "EMissive\\" 200.0)))

(event `HeistInteractionInterface.SetIsInFocus`
  (params (bIsInFocus :type Boolean))
  (bind _button_mid (`self.Button_MID`))
  (bind _output_get (set `self.bIsPowered` bIsInFocus))
  (if _output_get
    (`MaterialInstanceDynamic.SetScalarParameterValue` _button_mid "EMissive\\" 200.0)
    (else
      (`MaterialInstanceDynamic.SetScalarParameterValue` _button_mid "EMissive\\" 0.0)
      (message `HeistInteractionInterface.Interact` (`self.LinkedActor`)))))

(fn `UserConstructionScript`)