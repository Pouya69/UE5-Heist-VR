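; Test moving crate crane for the Heist game that carries a platform along a spline when switched on.
; Interact turns the linked light green, starts the machine sound and spline Timeline, and plays a cutscene on first start; InteractReset turns it red and stops both.
; A player overlap box fires a one-shot boarding cutscene.
; Player size changes switch the sound between proximity and 2D attenuation.
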(event `self.ReceiveBeginPlay`
  (bind _staticmeshcomponent (`StaticMeshActor.StaticMeshComponent` (`self.Light Ref`)))
  (`AudioComponent.Play` (`self.MachineSound`) 0.0)
  (bind _asheist_game_mode (cast `HeistGameMode` (`GameplayStatics.GetGameMode`)))
  (add `HeistGameMode.OnPlayerChangeSize` _asheist_game_mode (delegate `OnPlayerChangeSize_Event`))
  (`self.OnPlayerChangeSize_Event` "MEDIUM")
  (bind _returnvalue (`PrimitiveComponent.CreateDynamicMaterialInstance` _staticmeshcomponent 2 null "None"))
  (bind _output_get (set `self.MID_LightRef` _returnvalue))
  (`PrimitiveComponent.SetMaterial` _staticmeshcomponent 2 _output_get))

(event `OnPlayerChangeSize_Event`
  (params (NewPlayerSize :type "EHeistSize Enum" :default "TINY"))
  (set `AudioComponent.AttenuationSettings` (select `bool` (`|EnumEquality` NewPlayerSize "MEDIUM") :`false` "/Game/Audio_P1/System/ATT_2D.ATT_2D" :`true` "/Game/Audio_P1/System/ATT_Machine_Proximity.ATT_Machine_Proximity" :!type "SoundAttenuation Object Reference") (`self.MachineSound`)))

(event `self.ReceiveTick`
  (params (DeltaSeconds :type "Float (single-precision)")))

(event `HeistInteractionInterface.Interact`
  (bind _movingplatform1 (`self.MovingPlatform1`))
  (`|ExecutionSequence`
    (:`then_0`
      (`MaterialInstanceDynamic.SetVectorParameterValue` (`self.MID_LightRef`) "Color" (`KismetMathLibrary.MakeColor` 0.0 1.0)))
    (:`then_1`
      (set `self.Is On?` true)
      (`|ExecutionSequence`
        (:`then_0`
          (if (not (`self.Has Started First Time`))
            (`MovieSceneSequencePlayer.Play` (`LevelSequenceActor.SequencePlayer` (`self.Machine Cutscene Reference`)))))
        (:`then_1`
          (`AudioParameterControllerInterface.SetBoolParameter` (`self.MachineSound`) "Start_Machine" true)
          (set `self.Has Started First Time` true)
          (bind (_direction _spline_time_value) (`Timeline|Timeline` :!label _label)
            (:`Update`
              (bind (_returnvalue_location _returnvalue_rotation) (`KismetMathLibrary.BreakTransform` (`SplineComponent.GetTransformAtTime` (`self.Spline`) _spline_time_value "World" true false)))
              (`SceneComponent.K2_SetWorldTransform` _movingplatform1 (`KismetMathLibrary.MakeTransform` _returnvalue_location _returnvalue_rotation (`SceneComponent.K2_GetComponentScale` _movingplatform1)) false false))))))))

(event `HeistInteractionInterface.Interact_Reset`
  (`|ExecutionSequence`
    (:`then_0`
      (`MaterialInstanceDynamic.SetVectorParameterValue` (`self.MID_LightRef`) "Color" (`KismetMathLibrary.MakeColor` 1.0)))
    (:`then_1`
      (set `self.Is On?` false)
      (`AudioParameterControllerInterface.SetBoolParameter` (`self.MachineSound`) "StopMachine" true)
      (goto _label :!via `Stop`))))

(event `self.Player Overlap Box for Cutscene S017.OnComponentBeginOverlap`
  (params (OverlappedComponent :type "PrimitiveComponent Object Reference") (OtherActor :type "Actor Object Reference") (OtherComp :type "PrimitiveComponent Object Reference") (OtherBodyIndex :type Integer) (bFromSweep :type Boolean) (SweepResult :type "HitResult Structure (by ref)"))
  (if (`self.ActorHasTag` OtherActor "Player")
    (set `PrimitiveComponent.bGenerateOverlapEvents` false (`self.Player Overlap Box for Cutscene S017`))
    (`MovieSceneSequencePlayer.Play` (`LevelSequenceActor.SequencePlayer` (`self.S017 Cutscene Ref Player Got On Machine`)))))

(fn `Activate Moving Platform`
  (`HeistInteractionInterface.Interact`))

(fn `Dilation Platform`
  (set `self.CustomTimeDilation` 0.1))

(fn `GetAnchorSceneComponentForWheel`
  (returns (ReturnValue :type "SceneComponent Object Reference"))
  (return null))

(fn `GetCurrentSizeOfGameObject`
  (returns (ReturnValue :type "EHeistSize Enum"))
  (return "TINY"))

(fn `GetGrabComponents`
  (returns (OutGrabComponents :type "Array of HeistGrabComponent Object Reference") (ReturnValue :type Boolean))
  (return _ false))

(fn `GetHandAnimationType`
  (returns (ReturnValue :type "EHeistGrabHandState Enum"))
  (return "DEFAULT"))

(fn `GetIsInteractable`
  (returns (ReturnValue :type Boolean))
  (return (`self.Has Started First Time`)))

(fn `GetPhysicsConstraintComp`
  (returns (ReturnValue :type "PhysicsConstraintComponent Object Reference"))
  (return null))

(fn `IsGrabbable`
  (params (BoneHit :type Name))
  (returns (ReturnValue :type Boolean))
  (return (`self.Is On?`)))

(fn `IsRemoteGrabbable`
  (returns (ReturnValue :type Boolean))
  (return false))

(fn `RemoteGrab`
  (returns (ReturnValue :type Boolean))
  (return false))

(fn `UserConstructionScript`)