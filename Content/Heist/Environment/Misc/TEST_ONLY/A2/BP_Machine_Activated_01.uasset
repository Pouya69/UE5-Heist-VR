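; Test machine actor whose cube spins and changes its material when activated through Interact.
; BeginPlay gives the cube a dynamic material; Interact stamps Trigger_Time with the actor's age and enables Tick, which yaws the cube by Speed and CustomTimeDilation.
; InteractReset sets Trigger_Time far negative and disables Tick.
; Grab and interactable queries return false or defaults, so it cannot be grabbed.
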(event `self.ReceiveBeginPlay`
  (bind _rotating_cube (`self.Rotating Cube`))
  (bind _returnvalue (`PrimitiveComponent.CreateDynamicMaterialInstance` _rotating_cube 0 (`PrimitiveComponent.GetMaterial` _rotating_cube 0) "None"))
  (bind _output_get (set `self.MID` _returnvalue))
  (`PrimitiveComponent.SetMaterial` _rotating_cube 0 _output_get))

(event `self.ReceiveTick`
  (params (DeltaSeconds :type "Float (single-precision)"))
  (`SceneComponent.K2_AddLocalRotation` (`self.Rotating Cube`) (`KismetMathLibrary.MakeRotator` 0.0 0.0 (* DeltaSeconds (* (`self.Speed`) (`self.CustomTimeDilation`)))) false false))

(event `HeistInteractionInterface.Interact`
  (`MaterialInstanceDynamic.SetScalarParameterValue` (`self.MID`) "Trigger_Time" (`self.GetGameTimeSinceCreation`))
  (`self.SetActorTickEnabled` true))

(event `HeistInteractionInterface.Interact_Reset`
  (`MaterialInstanceDynamic.SetScalarParameterValue` (`self.MID`) "Trigger_Time" -999.0)
  (`self.SetActorTickEnabled` false))

(fn `GetAnchorSceneComponentForWheel`
  (returns (ReturnValue :type "SceneComponent Object Reference"))
  (return null))

(fn `GetCurrentSizeOfGameObject`
  (returns (ReturnValue :type "EHeistSize Enum"))
  (return "TINY"))

(fn `GetGrabComponents`
  (returns (OutGrabComponents :type "Array of HeistGrabComponent Object Reference") (ReturnValue :type Boolean))
  (return _ false))

(fn `GetHandAnimationType`
  (returns (ReturnValue :type "EHeistGrabHandState Enum"))
  (return "DEFAULT"))

(fn `GetIsInteractable`
  (returns (ReturnValue :type Boolean))
  (return false))

(fn `IsGrabbable`
  (params (BoneHit :type Name))
  (returns (ReturnValue :type Boolean))
  (return false))

(fn `IsRemoteGrabbable`
  (returns (ReturnValue :type Boolean))
  (return false))

(fn `RemoteGrab`
  (returns (ReturnValue :type Boolean))
  (return false))

(fn `UserConstructionScript`)