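; Elevator actor that travels along a spline, driven forward by Interact and back by InteractReset.
; A timeline, set to its end on BeginPlay, moves the whole actor at constant velocity, with the first reset reversing from the end.
; ElevatorStartGoing delays travel while sound parameters trigger door-close and move audio; finishing triggers the stop sound.
; Grab and interactable interface queries return false or defaults.
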(event `self.ReceiveBeginPlay`
  (bind (_direction _spline_time_value) (`Timeline|Timeline` :`NewTime` (`TimelineComponent.GetTimelineLength` (`self.Timeline`)) :!via `SetNewTime` :!label _label)
    (:`Update`
      (set `self.Current Time` _spline_time_value)
      (`self.K2_SetActorLocation` (`SplineComponent.GetLocationAtTime` (`self.Spline`) _spline_time_value "World" true)))
    (:`Finished`
      (`KismetSystemLibrary.Delay` 0.1)
      (`AudioParameterControllerInterface.SetBoolParameter` (`AmbientSound.AudioComponent` (`self.Elevator Sound Ref`)) "Stop_Move" true)
      (`KismetSystemLibrary.Delay` 1.6))))

(event `self.ReceiveTick`
  (params (DeltaSeconds :type "Float (single-precision)")))

(event `self.Interact`
  (if (not (`KismetMathLibrary.NearlyEqual_FloatFloat` (`self.Current Time`) 1.0 0.001))
    (`self.Elevator Start Going`
      (:`NewParam2`
        (goto _label)))))

(event `self.Interact_Reset`
  (if (not (`KismetMathLibrary.NearlyEqual_FloatFloat` (`self.Current Time`) 0.0 0.001))
    (`self.Elevator Start Going`
      (:`NewParam2`
        (if (`self.Has Started First Time`)
          (goto _label :!via `Reverse`)
          (else
            (set `self.Has Started First Time` true)
            (goto _label :!via `ReverseFromEnd`)))))))

(event `HeistInteractionInterface.ObjectSlowedDown`)

(event `HeistInteractionInterface.ObjectOutOfSlowMotion`)

(fn `GetAnchorSceneComponentForWheel`
  (returns (ReturnValue :type "SceneComponent Object Reference"))
  (return null))

(fn `GetCurrentSizeOfGameObject`
  (returns (ReturnValue :type "EHeistSize Enum"))
  (return "TINY"))

(fn `GetGrabComponents`
  (returns (OutGrabComponents :type "Array of HeistGrabComponent Object Reference") (ReturnValue :type Boolean))
  (return _ false))

(fn `GetHandAnimationType`
  (returns (ReturnValue :type "EHeistGrabHandState Enum"))
  (return "DEFAULT"))

(fn `GetIsInteractable`
  (returns (ReturnValue :type Boolean))
  (return false))

(fn `GetPhysicsConstraintComp`
  (returns (ReturnValue :type "PhysicsConstraintComponent Object Reference"))
  (return null))

(fn `Interactt`
  (`HeistInteractionInterface.Interact`))

(fn `IsGrabbable`
  (params (BoneHit :type Name))
  (returns (ReturnValue :type Boolean))
  (return false))

(fn `IsRemoteGrabbable`
  (returns (ReturnValue :type Boolean))
  (return false))

(fn `RemoteGrab`
  (returns (ReturnValue :type Boolean))
  (return false))

(fn `Reset Interact`
  (`HeistInteractionInterface.Interact_Reset`))

(fn `UserConstructionScript`)