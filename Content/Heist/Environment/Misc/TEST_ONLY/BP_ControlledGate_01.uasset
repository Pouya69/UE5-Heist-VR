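; Two-panel sliding gate that opens from an external normalized amount while held in focus and slides shut on release.
; SetAmount moves both meshes apart along world Y; Tick interpolates them closed, then disables itself when shut.
; First SetAmount plays an opening cutscene; closing plays a "did not reach in time" sequence unless CannotInteract flagged success.
; Slow-motion events scale custom time dilation and door sound pitch, slowing gate movement.
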(event `self.ReceiveTick`
  (params (DeltaSeconds :type "Float (single-precision)"))
  (bind _door_minmax_height_x (`KismetMathLibrary.BreakVector2D` (`self.Door_MinMax_Height`)))
  (bind (_door_minmax_height_x_2 _door_minmax_height_y) (`KismetMathLibrary.BreakVector2D` (`self.Door_MinMax_Height`)))
  (bind (_doorinitial_height_x _doorinitial_height_y _doorinitial_height_z) (`KismetMathLibrary.BreakVector` (`self.DoorInitial_Height`)))
  (bind (_doorinitial_height_02_x _doorinitial_height_02_y _doorinitial_height_02_z) (`KismetMathLibrary.BreakVector` (`self.DoorInitial_Height_02`)))
  (`|ExecutionSequence`
    (:`then_0`
      (if (not (`self.Is Grabbed`))
        (set `self.Current Normalized Amount` (`KismetMathLibrary.FInterpTo_Constant` (`self.Current Normalized Amount`) 0.0 (* DeltaSeconds (`self.CustomTimeDilation`)) (`self.Interp Speed`)))
        (bind _output_get (set `self.CurrentAmount` (`KismetMathLibrary.FInterpTo_Constant` (`self.CurrentAmount`) (`KismetMathLibrary.MapRangeClamped` (`self.Current Normalized Amount`) 0.0 1.0 _door_minmax_height_x_2 _door_minmax_height_y) (`GameplayStatics.GetWorldDeltaSeconds`) (* (`self.Interp Speed`) (`self.CustomTimeDilation`)))))
        (`|ExecutionSequence`
          (:`then_0`
            (`SceneComponent.K2_SetWorldLocation` (`self.StaticMesh`) (`KismetMathLibrary.MakeVector` _doorinitial_height_x (+ _doorinitial_height_y (* _output_get -1.0)) _doorinitial_height_z) true false))
          (:`then_1`
            (`SceneComponent.K2_SetWorldLocation` (`self.StaticMesh_02`) (`KismetMathLibrary.MakeVector` _doorinitial_height_02_x (+ _output_get _doorinitial_height_02_y) _doorinitial_height_02_z) true false))
          (:`then_2`
            (if (and (`KismetMathLibrary.NearlyEqual_FloatFloat` (`self.CurrentAmount`) _door_minmax_height_x 0.0001) (not (`self.Is Grabbed`)))
              (`self.Closed Gate Event`))))))))

(event `Closed Gate Event`
  (bind _door_sound (`self.Door Sound`))
  (bind _sequenceplayer (`LevelSequenceActor.SequencePlayer` (`self.Player Did Not Reach Gate In Time`)))
  (`AudioParameterControllerInterface.SetBoolParameter` _door_sound "Play_Impact" true)
  (`AudioParameterControllerInterface.SetBoolParameter` _door_sound "Stop_Slide" true)
  (`self.SetActorTickEnabled` false)
  (if (and (not (`self.Has Played Player Did Not Reach Gate In Time`)) (not (`MovieSceneSequencePlayer.IsPlaying` _sequenceplayer)))
    (`MovieSceneSequencePlayer.Stop` _sequenceplayer)
    (`MovieSceneSequencePlayer.Play` _sequenceplayer)))

(event `HeistInteractionInterface.CannotInteract`
  ; That means player reached in time we don't need to anymore.
  (set `self.Has Played Player Did Not Reach Gate In Time` true)
  (`self.ObjectOutOfSlowMotion`))

(event `self.ReceiveBeginPlay`
  (set `self.DoorInitial_Height` (`SceneComponent.K2_GetComponentLocation` (`self.StaticMesh`)))
  (set `self.DoorInitial_Height_02` (`SceneComponent.K2_GetComponentLocation` (`self.StaticMesh_02`)))
  (`AudioComponent.Play` (`self.Door Sound`) 0.0))

(event `HeistInteractionInterface.SetAmount`
  (params (NewAmount :type "Float (single-precision)"))
  (bind (_doorinitial_height_02_x _doorinitial_height_02_y _doorinitial_height_02_z) (`KismetMathLibrary.BreakVector` (`self.DoorInitial_Height_02`)))
  (bind (_doorinitial_height_x _doorinitial_height_y _doorinitial_height_z) (`KismetMathLibrary.BreakVector` (`self.DoorInitial_Height`)))
  (bind (_door_minmax_height_x _door_minmax_height_y) (`KismetMathLibrary.BreakVector2D` (`self.Door_MinMax_Height`)))
  (`|ExecutionSequence`
    (:`then_0`
      (if (not (`self.Has Started Door Cutscene`))
        (set `self.Has Started Door Cutscene` true)
        (`MovieSceneSequencePlayer.Play` (`LevelSequenceActor.SequencePlayer` (`self.Gate Door Open First Time Cutscene`)))))
    (:`then_1`
      (if (`self.Is Grabbed`)
        (bind _output_get (set `self.Current Normalized Amount` NewAmount))
        (bind _output_get_2 (set `self.CurrentAmount` (`KismetMathLibrary.FInterpTo_Constant` (`self.CurrentAmount`) (`KismetMathLibrary.MapRangeClamped` _output_get 0.0 1.0 _door_minmax_height_x _door_minmax_height_y) (* (`GameplayStatics.GetWorldDeltaSeconds`) (`self.CustomTimeDilation`)) (`self.Interp Speed`))))
        (`|ExecutionSequence`
          (:`then_0`
            (`SceneComponent.K2_SetWorldLocation` (`self.StaticMesh`) (`KismetMathLibrary.MakeVector` _doorinitial_height_x (+ (* _output_get_2 -1.0) _doorinitial_height_y) _doorinitial_height_z) true false))
          (:`then_1`
            (`SceneComponent.K2_SetWorldLocation` (`self.StaticMesh_02`) (`KismetMathLibrary.MakeVector` _doorinitial_height_02_x (+ _output_get_2 _doorinitial_height_02_y) _doorinitial_height_02_z) true false)))))))

(event `HeistInteractionInterface.Interact`)

(event `HeistInteractionInterface.ObjectSlowedDown`
  (set `self.CustomTimeDilation` (* (`self.CustomTimeDilation`) 0.3))
  (`AudioComponent.SetPitchMultiplier` (`self.Door Sound`) 0.3))

(event `HeistInteractionInterface.ObjectOutOfSlowMotion`
  (set `self.CustomTimeDilation` 1.0)
  (`AudioComponent.SetPitchMultiplier` (`self.Door Sound`) 1.0))

(event `HeistInteractionInterface.SetIsInFocus`
  (params (bIsInFocus :type Boolean))
  (set `self.Is Grabbed` bIsInFocus)
  (if bIsInFocus
    (`AudioParameterControllerInterface.SetBoolParameter` (`self.Door Sound`) "Play_Slide" true)
    (`self.SetActorTickEnabled` true)))

(fn `Dilation Test`
  (`HeistFunctionLibrary.SetTimeDilationOfObject` self 0.1 15.0))

(fn `GetAnchorSceneComponentForWheel`
  (returns (ReturnValue :type "SceneComponent Object Reference"))
  (return null))

(fn `GetCurrentSizeOfGameObject`
  (returns (ReturnValue :type "EHeistSize Enum"))
  (return "TINY"))

(fn `GetGrabComponents`
  (returns (OutGrabComponents :type "Array of HeistGrabComponent Object Reference") (ReturnValue :type Boolean))
  (return _ false))

(fn `GetHandAnimationType`
  (returns (ReturnValue :type "EHeistGrabHandState Enum"))
  (return "DEFAULT"))

(fn `GetIsInteractable`
  (returns (ReturnValue :type Boolean))
  (return false))

(fn `GetPhysicsConstraintComp`
  (returns (ReturnValue :type "PhysicsConstraintComponent Object Reference"))
  (return null))

(fn `IsGrabbable`
  (params (BoneHit :type Name))
  (returns (ReturnValue :type Boolean))
  (return false))

(fn `IsRemoteGrabbable`
  (returns (ReturnValue :type Boolean))
  (return false))

(fn `RemoteGrab`
  (returns (ReturnValue :type Boolean))
  (return false))

(fn `Set Amount half`
  (`HeistInteractionInterface.SetAmount` 0.5))

(fn `Set Amount one`
  (`HeistInteractionInterface.SetAmount` 1.0))

(fn `Set Amount Zero`
  (`HeistInteractionInterface.SetAmount` 0.0))

(fn `Set In Focus`
  (`HeistInteractionInterface.SetIsInFocus` true))

(fn `Set Not In Focus`
  (`HeistInteractionInterface.SetIsInFocus` false))

(fn `UserConstructionScript`)