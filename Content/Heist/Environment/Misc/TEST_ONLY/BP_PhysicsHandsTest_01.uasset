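; Test actor for physics-based two-handed grabbing, using left and right spheres as stand-in hands.
; GrabTwoHands checks that the GrabbableTwohandTest grab component's type is HANDED, then binds each sphere to its primitive through that side's physics constraint.
; The event graph is inactive, holding only disconnected earlier versions of the constraint setup, and nothing in this Blueprint calls GrabTwoHands.
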(event `self.ReceiveBeginPlay`)

(fn `Grab Two Hands`
  (bind _primitivecomponent (`HeistGrabComponent.PrimitiveComponent` (`Grabbable.GrabComponent` (`self.Grabbable_Twohand_Test`))))
  (if (`|EnumEquality` (`HeistGrabComponent.GrabTypeBase` (`Grabbable.GrabComponent` (`self.Grabbable_Twohand_Test`))) "TWO_HANDED")
    (`PhysicsConstraintComponent.SetConstrainedComponents` (`self.PhysicsConstraint_L`) (`self.Sphere_L`) "None" _primitivecomponent "None")
    (`PhysicsConstraintComponent.SetConstrainedComponents` (`self.PhysicsConstraint_R`) (`self.Sphere_R`) "None" _primitivecomponent "None")))

(fn `UserConstructionScript`)