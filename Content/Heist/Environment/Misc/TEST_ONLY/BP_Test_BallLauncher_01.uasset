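; Test launcher actor that fires small grabbable cubes from its Arrow component.
; On Interact, it spawns a scaled-down cube at the arrow's transform with a short lifespan and applies a velocity-change impulse along the arrow's forward vector.
; SetAmount stores a strength value that scales the extra speed added to the base velocity.
; Grab and interactable queries return false, and TestInteract also triggers a launch.
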(event `HeistInteractionInterface.Interact`
  (bind (_returnvalue_location _returnvalue_rotation) (`KismetMathLibrary.BreakTransform` (`SceneComponent.K2_GetComponentToWorld` (`self.Arrow`))))
  (bind _returnvalue (`|SpawnActorFromClass` "/Game/Heist/Environment/Grabbable_SmallCube.Grabbable_SmallCube_C" (`KismetMathLibrary.MakeTransform` _returnvalue_location _returnvalue_rotation (0.3 0.3 0.3)) "AlwaysSpawn" "MultiplyWithRoot" null self))
  (`self.SetLifeSpan` _returnvalue 5.0)
  (`PrimitiveComponent.AddImpulse` (`HeistGrabComponent.PrimitiveComponent` (`Grabbable.GrabComponent` _returnvalue)) (* (`SceneComponent.GetForwardVector` (`self.Arrow`)) (+ (`self.BaseVelocity`) (* (`self.Strength`) (`self.Max_Strength_Velocity`)))) "None" true))

(event `HeistInteractionInterface.SetAmount`
  (params (NewAmount :type "Float (single-precision)"))
  (set `self.Strength` NewAmount))

(fn `GetGrabComponents`
  (returns (OutGrabComponents :type "Array of HeistGrabComponent Object Reference") (ReturnValue :type Boolean))
  (return _ false))

(fn `GetHandAnimationType`
  (returns (ReturnValue :type "EHeistGrabHandState Enum"))
  (return "DEFAULT"))

(fn `GetIsInteractable`
  (returns (ReturnValue :type Boolean))
  (return false))

(fn `IsGrabbable`
  (params (BoneHit :type Name))
  (returns (ReturnValue :type Boolean))
  (return false))

(fn `IsRemoteGrabbable`
  (returns (ReturnValue :type Boolean))
  (return false))

(fn `RemoteGrab`
  (returns (ReturnValue :type Boolean))
  (return false))

(fn `Test_Interact`
  (`HeistInteractionInterface.Interact`))

(fn `UserConstructionScript`)