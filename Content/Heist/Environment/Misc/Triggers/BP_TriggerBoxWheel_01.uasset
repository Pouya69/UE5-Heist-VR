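; Trigger volume that receives a detachable HeistWheel and hooks it up to a linked actor.
; When a component tagged Detachable overlaps it, the trigger switches off its overlap events, even if the wheel is then rejected.
; A wheel without a linked actor receives the trigger's LinkedActor and attaches to the optional anchor actor's component, falling back to the trigger's collision component.
; The valve puzzle sound is left unconnected.
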(event `self.CollisionComponent.OnComponentBeginOverlap`
  (params (OverlappedComponent :type "PrimitiveComponent Object Reference") (OtherActor :type "Actor Object Reference") (OtherComp :type "PrimitiveComponent Object Reference") (OtherBodyIndex :type Integer) (bFromSweep :type Boolean) (SweepResult :type "HitResult Structure (by ref)"))
  (bind _new_anchor_point_for_wheel (`self.New Anchor Point For Wheel`))
  (if (`ActorComponent.ComponentHasTag` OtherComp "Detachable")
    (set `PrimitiveComponent.bGenerateOverlapEvents` false (`self.CollisionComponent`))
    (bind _asheist_wheel (cast `HeistWheel` OtherActor))
    (`HeistWheel.LinkedActor` _asheist_wheel ; Only if does not have one.
      (:`then`)
      (:`else`
        (`|ExecutionSequence`
          (:`then_0`
            (`HeistWheel.ChangeLinkedActor` _asheist_wheel (`self.Linked Actor`)))
          (:`then_1`
            (`/Engine/EditorBlueprintResources/StandardMacros.IsValid` _new_anchor_point_for_wheel
              (:`Is Valid`
                (bind _returnvalue (message `HeistInteractionInterface.GetAnchorSceneComponentForWheel` _new_anchor_point_for_wheel))
                (`HeistWheel.AttachToNewAnchorPoint` _asheist_wheel _returnvalue))
              (:`Is Not Valid`
                (`HeistWheel.AttachToNewAnchorPoint` _asheist_wheel (`self.CollisionComponent`))))))))))

(fn `UserConstructionScript`)