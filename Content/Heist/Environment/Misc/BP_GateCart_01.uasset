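; Heist environment gate that moves a cube along a spline when its focus state changes.
; Gaining focus plays a timeline that positions the cube by constant-velocity spline sampling, and losing focus reverses it.
; A box trigger halts the reverse movement on overlap and reverses the timeline whenever it empties, without checking focus.
; Grab and interaction functions are stubs reporting it as neither grabbable nor interactable.
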(event `HeistInteractionInterface.SetIsInFocus`
  (params (bIsInFocus :type Boolean))
  (if bIsInFocus
    (bind (_direction _gate_height_track) (`Timeline|Gate Timeline` :!label _label)
      (:`Update`
        (`SceneComponent.K2_SetWorldLocation` (`self.Cube`) (`SplineComponent.GetLocationAtTime` (`self.Spline`) _gate_height_track "World" true) false false)))
    (else
      (goto _label :!via `Reverse`))))

(event `self.Box.OnComponentBeginOverlap`
  (params (OverlappedComponent :type "PrimitiveComponent Object Reference") (OtherActor :type "Actor Object Reference") (OtherComp :type "PrimitiveComponent Object Reference") (OtherBodyIndex :type Integer) (bFromSweep :type Boolean) (SweepResult :type "HitResult Structure (by ref)"))
  (if (`TimelineComponent.IsReversing` (`self.Gate Timeline`))
    (goto _label :!via `Stop`)))

(event `self.Box.OnComponentEndOverlap`
  (params (OverlappedComponent :type "PrimitiveComponent Object Reference") (OtherActor :type "Actor Object Reference") (OtherComp :type "PrimitiveComponent Object Reference") (OtherBodyIndex :type Integer))
  (if (`KismetArrayLibrary.Array_IsEmpty` (`PrimitiveComponent.GetOverlappingActors` (`self.Box`) null))
    (goto _label :!via `Reverse`)))

(fn `GetAnchorSceneComponentForWheel`
  (returns (ReturnValue :type "SceneComponent Object Reference"))
  (return null))

(fn `GetCurrentSizeOfGameObject`
  (returns (ReturnValue :type "EHeistSize Enum"))
  (return "TINY"))

(fn `GetGrabComponents`
  (returns (OutGrabComponents :type "Array of HeistGrabComponent Object Reference") (ReturnValue :type Boolean))
  (return _ false))

(fn `GetHandAnimationType`
  (returns (ReturnValue :type "EHeistGrabHandState Enum"))
  (return "DEFAULT"))

(fn `GetIsInteractable`
  (returns (ReturnValue :type Boolean))
  (return false))

(fn `GetPhysicsConstraintComp`
  (returns (ReturnValue :type "PhysicsConstraintComponent Object Reference"))
  (return null))

(fn `IsGrabbable`
  (params (BoneHit :type Name))
  (returns (ReturnValue :type Boolean))
  (return false))

(fn `IsRemoteGrabbable`
  (returns (ReturnValue :type Boolean))
  (return false))

(fn `RemoteGrab`
  (returns (ReturnValue :type Boolean))
  (return false))

(fn `UserConstructionScript`)