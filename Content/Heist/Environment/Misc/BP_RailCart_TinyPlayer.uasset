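; Rail cart that carries the player along a spline, shown only at tiny player size when the cart's own size is TINY.
; Overlapping the collision box teleports a tagged player to the seat point and stores the reference.
; With a player stored, Interact plays a timeline moving the cart at constant velocity, and InteractReset reverses it.
; Messages report boarding and leaving; object-carrying logic is disconnected.
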(event `self.ReceiveBeginPlay`
  (`self.K2_AttachToComponent` (`self.LeverRef`) (`self.MainMoving_Part`) "None" "KeepWorld" "KeepWorld" "KeepWorld" true)
  (if (`|EnumEquality` (`self.Current Size`) "TINY")
    (bind _asheist_game_mode (cast `HeistGameMode` (`GameplayStatics.GetGameMode`)))
    (add `HeistGameMode.OnPlayerChangeSize` _asheist_game_mode (delegate `OnPlayerChangeSize_Event`))
    (`self.OnPlayerChangeSize_Event` "MEDIUM")))

(event `OnPlayerChangeSize_Event`
  (params (NewPlayerSize :type "EHeistSize Enum" :default "TINY"))
  (`SceneComponent.SetVisibility` (`self.MainMoving_Part`) (`|EnumEquality` NewPlayerSize "TINY") true))

(event `self.CollisionBox.OnComponentBeginOverlap`
  (params (OverlappedComponent :type "PrimitiveComponent Object Reference") (OtherActor :type "Actor Object Reference") (OtherComp :type "PrimitiveComponent Object Reference") (OtherBodyIndex :type Integer) (bFromSweep :type Boolean) (SweepResult :type "HitResult Structure (by ref)"))
  (`self.PlayerRefSOFT`
    (:`then`)
    (:`else`
      (if (`self.ActorHasTag` OtherActor "Player")
        (bind _output_get (set `self.PlayerRefSOFT` OtherActor))
        (message `HeistPlayerInterface.TeleportPlayerTo` _output_get (`SceneComponent.K2_GetComponentLocation` (`self.Player Location`)))))))

(event `self.SetIsInFocus`
  (params (bIsInFocus :type Boolean)))

(event `self.CollisionBox.OnComponentEndOverlap`
  (params (OverlappedComponent :type "PrimitiveComponent Object Reference") (OtherActor :type "Actor Object Reference") (OtherComp :type "PrimitiveComponent Object Reference") (OtherBodyIndex :type Integer))
  (bind _playerrefsoft (`self.PlayerRefSOFT`))
  (if (== OtherActor _playerrefsoft)
    (message `HeistPlayerInterface.GotInCart` _playerrefsoft false)
    (set `self.PlayerRefSOFT` null)))

(event `self.SetNewSizeTo`
  (params (NewSize :type "EHeistSize Enum" :default "TINY"))
  (set `self.Current Size` NewSize))

(event `self.Interact`
  (bind _playerrefsoft (`self.PlayerRefSOFT`)
    (:`then`
      (message `HeistPlayerInterface.GotInCart` _playerrefsoft true)
      (if (`self.Has Started`)
        (bind (_direction _cart_track) (`Timeline|Railcart Timeline` :!label _label)
          (:`Update`
            (`SceneComponent.K2_SetWorldLocation` (`self.MainMoving_Part`) (`SplineComponent.GetLocationAtTime` (`self.Spline`) _cart_track "World" true) false false))
          (:`Finished`
            (bind _playerrefsoft_2 (`self.PlayerRefSOFT`)
              (:`then`
                (message `HeistPlayerInterface.GotInCart` _playerrefsoft_2 false)
                (`self.K2_DetachFromActor` _playerrefsoft_2 "KeepWorld" "KeepWorld" "KeepWorld"))
              (:`else`))))
        (else
          (set `self.Has Started` true)
          (goto _label))))
    (:`else`)))

(event `self.Interact_Reset`
  (bind _playerrefsoft (`self.PlayerRefSOFT`)
    (:`then`
      (message `HeistPlayerInterface.GotInCart` _playerrefsoft true)
      (if (`self.Has Started`)
        (goto _label :!via `Reverse`)
        (else
          (set `self.Has Started` true)
          (goto _label :!via `Reverse`))))
    (:`else`)))

(fn `Dilation Test`
  (`HeistFunctionLibrary.SetTimeDilationOfObject` self 0.1 10.0))

(fn `GetAnchorSceneComponentForWheel`
  (returns (ReturnValue :type "SceneComponent Object Reference"))
  (return null))

(fn `GetCurrentSizeOfGameObject`
  (returns (ReturnValue :type "EHeistSize Enum"))
  (return (`self.Current Size`)))

(fn `GetGrabComponents`
  (returns (OutGrabComponents :type "Array of HeistGrabComponent Object Reference") (ReturnValue :type Boolean))
  (return _ false))

(fn `GetHandAnimationType`
  (returns (ReturnValue :type "EHeistGrabHandState Enum"))
  (return "DEFAULT"))

(fn `GetIsInteractable`
  (returns (ReturnValue :type Boolean))
  (return false))

(fn `GetPhysicsConstraintComp`
  (returns (ReturnValue :type "PhysicsConstraintComponent Object Reference"))
  (return null))

(fn `Interact Reset Test`
  (`HeistInteractionInterface.Interact_Reset`))

(fn `Interact Test`
  (`HeistInteractionInterface.Interact`))

(fn `IsGrabbable`
  (params (BoneHit :type Name))
  (returns (ReturnValue :type Boolean))
  (return false))

(fn `IsRemoteGrabbable`
  (returns (ReturnValue :type Boolean))
  (return false))

(fn `RemoteGrab`
  (returns (ReturnValue :type Boolean))
  (return false))

(fn `UserConstructionScript`)