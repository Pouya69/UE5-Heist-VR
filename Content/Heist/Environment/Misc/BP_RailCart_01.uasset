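; Rail cart that travels along a spline: Interact plays a timeline that positions the moving part, and InteractReset reverses it.
; Components overlapping its collision box are mutually ignored for movement with the cart until they leave.
; A cart that starts tiny listens to the game mode's player-size changes, showing its moving part only while the player is tiny.
; Logic for attaching objects to the cart is present but disconnected.
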(event `self.ReceiveBeginPlay`
  (if (`|EnumEquality` (`self.Current Size`) "TINY")
    (bind _asheist_game_mode (cast `HeistGameMode` (`GameplayStatics.GetGameMode`)))
    (add `HeistGameMode.OnPlayerChangeSize` _asheist_game_mode (delegate `OnPlayerChangeSize_Event`))
    (`self.OnPlayerChangeSize_Event` "MEDIUM")))

(event `OnPlayerChangeSize_Event`
  (params (NewPlayerSize :type "EHeistSize Enum" :default "TINY"))
  (`SceneComponent.SetVisibility` (`self.MainMoving_Part`) (`|EnumEquality` NewPlayerSize "TINY") true))

(event `self.CollisionBox.OnComponentBeginOverlap`
  (params (OverlappedComponent :type "PrimitiveComponent Object Reference") (OtherActor :type "Actor Object Reference") (OtherComp :type "PrimitiveComponent Object Reference") (OtherBodyIndex :type Integer) (bFromSweep :type Boolean) (SweepResult :type "HitResult Structure (by ref)"))
  (`PrimitiveComponent.IgnoreActorWhenMoving` OtherComp self true)
  (`PrimitiveComponent.IgnoreComponentWhenMoving` (`self.MainMoving_Part`) OtherComp true))

(event `HeistInteractionInterface.SetIsInFocus`
  (params (bIsInFocus :type Boolean)))

(event `self.CollisionBox.OnComponentEndOverlap`
  (params (OverlappedComponent :type "PrimitiveComponent Object Reference") (OtherActor :type "Actor Object Reference") (OtherComp :type "PrimitiveComponent Object Reference") (OtherBodyIndex :type Integer))
  (`PrimitiveComponent.IgnoreActorWhenMoving` OtherComp self false)
  (`PrimitiveComponent.IgnoreComponentWhenMoving` (`self.MainMoving_Part`) OtherComp false))

(event `HeistInteractionInterface.Interact`
  (if (`self.Has Started`)
    (bind (_direction _cart_track) (`Timeline|Railcart Timeline` :!label _label)
      (:`Update`
        (bind _sweephitresult (`SceneComponent.K2_SetWorldLocation` (`self.MainMoving_Part`) (`SplineComponent.GetLocationAtTime` (`self.Spline`) _cart_track "World" true) false false))))
    (else
      (set `self.Has Started` true)
      (goto _label))))

(event `HeistInteractionInterface.Interact_Reset`
  (if (`self.Has Started`)
    (goto _label :!via `Reverse`)
    (else
      (set `self.Has Started` true)
      (goto _label :!via `Reverse`))))

(event `HeistInteractionInterface.SetNewSizeTo`
  (params (NewSize :type "EHeistSize Enum" :default "TINY"))
  (set `self.Current Size` NewSize))

(fn `Dilation Test`
  (`HeistFunctionLibrary.SetTimeDilationOfObject` self 0.1 10.0))

(fn `GetAnchorSceneComponentForWheel`
  (returns (ReturnValue :type "SceneComponent Object Reference"))
  (return null))

(fn `GetCurrentSizeOfGameObject`
  (returns (ReturnValue :type "EHeistSize Enum"))
  (return (`self.Current Size`)))

(fn `GetGrabComponents`
  (returns (OutGrabComponents :type "Array of HeistGrabComponent Object Reference") (ReturnValue :type Boolean))
  (return _ false))

(fn `GetHandAnimationType`
  (returns (ReturnValue :type "EHeistGrabHandState Enum"))
  (return "DEFAULT"))

(fn `GetIsInteractable`
  (returns (ReturnValue :type Boolean))
  (return false))

(fn `GetPhysicsConstraintComp`
  (returns (ReturnValue :type "PhysicsConstraintComponent Object Reference"))
  (return null))

(fn `Interact Reset Test`
  (`HeistInteractionInterface.Interact_Reset`))

(fn `Interact Test`
  (`HeistInteractionInterface.Interact`))

(fn `IsGrabbable`
  (params (BoneHit :type Name))
  (returns (ReturnValue :type Boolean))
  (return false))

(fn `IsRemoteGrabbable`
  (returns (ReturnValue :type Boolean))
  (return false))

(fn `RemoteGrab`
  (returns (ReturnValue :type Boolean))
  (return false))

(fn `UserConstructionScript`)