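; BP_WheelDetachable_04 is a grabbable detachable wheel prop for the Heist game, built from base, wheel and handle meshes.
; Grabbing it marks it remote-grabbable, and focus toggles an overlay highlight on all three meshes.
; It listens to the game mode's player-size change and, when unlinked and remote-grabbable, briefly suspends physics simulation on the base mesh before re-enabling it.
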(event `self.ReceiveBeginPlay`
  (bind _asheist_game_mode (cast `HeistGameMode` (`GameplayStatics.GetGameMode`)))
  (add `HeistGameMode.OnPlayerChangeSize` _asheist_game_mode (delegate `OnPlayerChangeSize_Event`)))

(event `OnPlayerChangeSize_Event`
  (params (NewPlayerSize :type "EHeistSize Enum" :default "TINY"))
  (bind _basemeshcomponent (`self.BaseMeshComponent`))
  (`self.LinkedActor`
    (:`then`)
    (:`else`
      (if (`self.bIsRemoteGrabbable`)
        (`PrimitiveComponent.SetSimulatePhysics` _basemeshcomponent false)
        (`KismetSystemLibrary.Delay` 0.8)
        (`PrimitiveComponent.SetSimulatePhysics` _basemeshcomponent true)))))

(event `self.GrabComponent.OnGrabbed`
  (params (GrabbedComponent :type "HeistGrabComponent Object Reference") (MotionControllerRef :type "HeistMotionControllerComponent Object Reference"))
  (`self.SetIsRemoteGrabbable` true))

(event `HeistInteractionInterface.SetIsInFocus`
  (params (bIsInFocus :type Boolean))
  (`MeshComponent.SetOverlayMaterial` (`self.BaseMeshComponent`) (select `bool` bIsInFocus :`true` (`self.InFocusMaterial`)))
  (`MeshComponent.SetOverlayMaterial` (`self.WheelMeshComponent`) (select `bool` bIsInFocus :`true` (`self.InFocusMaterial`)))
  (`MeshComponent.SetOverlayMaterial` (`self.HandleMeshComponent`) (select `bool` bIsInFocus :`true` (`self.InFocusMaterial`))))

(fn `GetGrabComponents`
  (returns (OutGrabComponents :type "Array of HeistGrabComponent Object Reference") (ReturnValue :type Boolean))
  (return (`|MakeArray` (`self.GrabComponent`)) true))

(fn `UserConstructionScript`)