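; Heist hallway door Blueprint, named as an outward-opening test variant, that becomes physics-driven when interacted with.
; Interact enables physics simulation on the door mesh and binds it to DoorConstraint as the first constrained component, without calling the parent Interact.
; ToggleOpenDoor passes the inverse of the mesh's simulation state to OpenCloseDoor, which is not defined here.
; TestInteract simply triggers Interact.
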(event `self.ReceiveTick`
  (params (DeltaSeconds :type "Float (single-precision)")))

(event `HeistInteractionInterface.Interact`
  (bind _doormeshcomponent (`self.DoorMeshComponent`))
  (`PrimitiveComponent.SetSimulatePhysics` _doormeshcomponent true)
  (`PhysicsConstraintComponent.SetConstrainedComponents` (`self.DoorConstraint`) _doormeshcomponent "None" null "None"))

(fn `Test Interact`
  (`HeistInteractionInterface.Interact`))

(fn `ToggleOpenDoor`
  (`self.OpenCloseDoor` (not (`SceneComponent.IsSimulatingPhysics` (`self.DoorMeshComponent`) "None"))))

(fn `UserConstructionScript`)