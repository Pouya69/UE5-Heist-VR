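; BP_DoorTest_Outwards_01 is a test door that triggers the S002 cutscene on its first interaction.
; BeginPlay disables mesh physics and breaks the door constraint.
; The first Interact enables physics, sets the mesh as a constrained component and plays the cutscene's sequence, with a flag blocking repeats.
; Helper functions toggle OpenCloseDoor from the mesh's physics state and call Interact for testing.
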(event `self.ReceiveBeginPlay`
  (`PrimitiveComponent.SetSimulatePhysics` (`self.DoorMeshComponent`) false)
  (`PhysicsConstraintComponent.BreakConstraint` (`self.DoorConstraint`)))

(event `self.ReceiveTick`
  (params (DeltaSeconds :type "Float (single-precision)")))

(event `HeistInteractionInterface.Interact`
  (bind _doormeshcomponent (`self.DoorMeshComponent`))
  (if (not (`self.Has Started Cutscene`))
    (set `self.Has Started Cutscene` true)
    (`PrimitiveComponent.SetSimulatePhysics` _doormeshcomponent true)
    (`PhysicsConstraintComponent.SetConstrainedComponents` (`self.DoorConstraint`) _doormeshcomponent "None" null "None")
    (`MovieSceneSequencePlayer.Play` (`LevelSequenceActor.SequencePlayer` (`self.S002_Cutscene_Reference`)))))

(fn `Test Interact`
  (`HeistInteractionInterface.Interact`))

(fn `ToggleOpenDoor`
  (`self.OpenCloseDoor` (not (`SceneComponent.IsSimulatingPhysics` (`self.DoorMeshComponent`) "None"))))

(fn `UserConstructionScript`)