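; Heist environment button that triggers a linked SizeChangeMachine to change the player's size.
; BeginPlay gives the moving button mesh a dynamic material instance to drive its emissive glow.
; Interact switches the glow off and calls the machine, and the glow returns when the button reaches its starting point.
; Logic caching a linked actor's light component is present but never runs.
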(event `self.ReceiveBeginPlay`
  (bind _buttonmovingmeshcomponent (`self.ButtonMovingMeshComponent`))
  (bind _returnvalue (`PrimitiveComponent.CreateDynamicMaterialInstance` _buttonmovingmeshcomponent 0 (`PrimitiveComponent.GetMaterial` _buttonmovingmeshcomponent 0) "None"))
  (bind _output_get (set `self.Button_MID` _returnvalue))
  (`PrimitiveComponent.SetMaterial` _buttonmovingmeshcomponent 0 _output_get))

(event `HeistInteractionInterface.Interact`
  (`MaterialInstanceDynamic.SetScalarParameterValue` (`self.Button_MID`) "EMissive\\" 0.0)
  (bind _assize_change_machine (cast `SizeChangeMachine` (`self.LinkedActor`)))
  (`SizeChangeMachine.ChangePlayerSize` _assize_change_machine))

(event `self.ButtonAtStartingPoint`
  (`MaterialInstanceDynamic.SetScalarParameterValue` (`self.Button_MID`) "EMissive\\" 200.0))

(fn `UserConstructionScript`)