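; Interactable button Blueprint that changes the player's size to medium when pressed.
; On BeginPlay it creates a dynamic material for the moving button mesh and caches the linked actor's root light component, which goes unused in these graphs.
; Interact switches off the emissive glow and sends a size-change message to the player pawn.
; The glow is restored when the button is back at its starting point.
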(event `self.ReceiveBeginPlay`
  (bind _buttonmovingmeshcomponent (`self.ButtonMovingMeshComponent`))
  (bind _returnvalue (`PrimitiveComponent.CreateDynamicMaterialInstance` _buttonmovingmeshcomponent 0 (`PrimitiveComponent.GetMaterial` _buttonmovingmeshcomponent 0) "None"))
  (bind _output_get (set `self.Button_MID` _returnvalue))
  (`PrimitiveComponent.SetMaterial` _buttonmovingmeshcomponent 0 _output_get)
  (bind _linkedactor (`self.LinkedActor`)
    (:`then`
      (bind _aslight_component (cast `LightComponent` (`Actor.RootComponent` _linkedactor)))
      (set `self.Light_LinkedActor` _aslight_component))
    (:`else`)))

(event `HeistInteractionInterface.Interact`
  (`MaterialInstanceDynamic.SetScalarParameterValue` (`self.Button_MID`) "EMissive\\" 0.0)
  (message `HeistPlayerInterface.ChangeSize` (`GameplayStatics.GetPlayerPawn` 0) "MEDIUM" (0.0 0.0 0.0)))

(event `self.ButtonAtStartingPoint`
  (`MaterialInstanceDynamic.SetScalarParameterValue` (`self.Button_MID`) "EMissive\\" 200.0))

(fn `UserConstructionScript`)