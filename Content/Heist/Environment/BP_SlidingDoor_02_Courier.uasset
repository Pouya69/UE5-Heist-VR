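; BP_SlidingDoor_02_Courier is a Heist sliding door that cannot be grabbed and starts a referenced cutscene sequence the first time it is interacted with.
; It begins with its physics constraint broken and simulation off.
; SetIsInteractable force-releases it, then either disables physics and collision when true, or restores both and re-attaches the constraint when false.
; Disconnected leftovers cover slide limits, a shove force and courier cutscene interruption.
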(event `self.ReceiveBeginPlay`
  (`PhysicsConstraintComponent.BreakConstraint` (`self.DoorPhysicsConstraint`))
  (`PrimitiveComponent.SetSimulatePhysics` (`self.BaseMeshComponent`) false))

(event `HeistInteractionInterface.ReleaseConstraintFromAnchor`
  (params (ReleasedConstraintComp :type "PhysicsConstraintComponent Object Reference")))

(event `HeistInteractionInterface.Interact`
  (if (not (`self.Has Started Cutscene`))
    (set `self.Has Started Cutscene` true)
    (`KismetSystemLibrary.DelayUntilNextTick`)
    (`MovieSceneSequencePlayer.Play` (`LevelSequenceActor.SequencePlayer` (`self.Cutscene Reference`)))))

(event `HeistInteractionInterface.SetIsInteractable`
  (params (bIsInteractable :type Boolean))
  (bind _basemeshcomponent (`self.BaseMeshComponent`))
  (bind _doorphysicsconstraint (`self.DoorPhysicsConstraint`))
  (`self.ForceRelease`)
  (if bIsInteractable
    (`PhysicsConstraintComponent.BreakConstraint` _doorphysicsconstraint)
    (`PrimitiveComponent.SetSimulatePhysics` _basemeshcomponent false)
    (`PrimitiveComponent.SetCollisionEnabled` _basemeshcomponent "NoCollision")
    (else
      (`PrimitiveComponent.SetCollisionEnabled` _basemeshcomponent "QueryAndPhysics")
      (`PrimitiveComponent.SetSimulatePhysics` _basemeshcomponent true)
      (`KismetSystemLibrary.DelayUntilNextTick`)
      (`PrimitiveComponent.WakeRigidBody` _basemeshcomponent "None")
      (`PhysicsConstraintComponent.SetConstrainedComponents` _doorphysicsconstraint _basemeshcomponent "None" null "None"))))

(fn `Interact Test`
  (`HeistInteractionInterface.Interact`))

(fn `IsGrabbable`
  (params (BoneHit :type Name))
  (returns (ReturnValue :type Boolean))
  (return false))

(fn `UserConstructionScript`)