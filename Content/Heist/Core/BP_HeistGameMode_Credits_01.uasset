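; Game mode for the Heist game, apparently for its credits level.
; On BeginPlay it sets the anti-aliasing method to 3 (MSAA) through a console command.
; ChangePlayerSize only forwards the new size to the parent implementation.
; Disconnected leftover nodes would lower overall scalability and print the names of actors with near-zero scale, but they never run.
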(event `self.ReceiveBeginPlay`
  (`KismetSystemLibrary.ExecuteConsoleCommand` "r.AntiAliasingMethod 3" null))

(event `self.ChangePlayerSize`
  (params (NewPlayerSize :type "EHeistSize Enum" :default "TINY"))
  (`parent.ChangePlayerSize` NewPlayerSize))

(fn `UserConstructionScript`)