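; BP_Courier_TESTT_01 is a test Blueprint for the Courier character that feeds a look-at target to its animation Blueprint.
; On BeginPlay and every Tick, it casts the skeletal mesh's anim instance to ABP_Courier_03_Test_01.
; It then copies CustomLocationToLookAt's actor location into PlayerCameraLocation, so a chosen actor supplies that location, and PlayerAlpha into UsePlayerRotationAlpha.
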(event `self.ReceiveBeginPlay`
  (bind _asabp_courier_03_test_01 (cast `/Game/Assets/Characters/MainCharacter/6/ABP_Courier_03_Test_01` (`SkeletalMeshComponent.GetAnimInstance` (`self.SkeletalMesh`))))
  (set `/Game/Assets/Characters/MainCharacter/6/ABP_Courier_03_Test_01.Player_Camera_Location` (`self.K2_GetActorLocation` (`self.Custom_Location_To_Look_At`)) _asabp_courier_03_test_01)
  (set `/Game/Assets/Characters/MainCharacter/6/ABP_Courier_03_Test_01.Use_Player_Rotation_Alpha` (`self.PlayerAlpha`) _asabp_courier_03_test_01))

(event `self.ReceiveTick`
  (params (DeltaSeconds :type "Float (single-precision)"))
  (bind _asabp_courier_03_test_01 (cast `/Game/Assets/Characters/MainCharacter/6/ABP_Courier_03_Test_01` (`SkeletalMeshComponent.GetAnimInstance` (`self.SkeletalMesh`))))
  (set `/Game/Assets/Characters/MainCharacter/6/ABP_Courier_03_Test_01.Player_Camera_Location` (`self.K2_GetActorLocation` (`self.Custom_Location_To_Look_At`)) _asabp_courier_03_test_01)
  (set `/Game/Assets/Characters/MainCharacter/6/ABP_Courier_03_Test_01.Use_Player_Rotation_Alpha` (`self.PlayerAlpha`) _asabp_courier_03_test_01))

(fn `UserConstructionScript`)