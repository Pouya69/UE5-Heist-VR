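; Test courier character that feeds its Animation Blueprint a look-at position, by default the VR player's camera.
; BeginPlay falls back to the VRPawn_HandTrace camera when no custom look-at component is set.
; BeginPlay and Tick push that component's world location and PlayerAlpha, as the rotation blend alpha, into ABP_Courier_03_Test_01.
; Death montage playback nodes are present but unconnected.
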(event `self.ReceiveBeginPlay`
  (`|ExecutionSequence`
    (:`then_0`
      (`self.Custom_Location_To_Look_At`
        (:`then`)
        (:`else`
          (bind _asvrpawn_hand_trace (cast `/Game/Heist/Player/VRPawn_HandTrace` (`GameplayStatics.GetPlayerPawn` 0)))
          (set `self.Custom_Location_To_Look_At` (`/Game/Heist/Player/VRPawn_HandTrace.Camera` _asvrpawn_hand_trace)))))
    (:`then_1`
      (bind _asabp_courier_03_test_01 (cast `/Game/Assets/Characters/MainCharacter/6/ABP_Courier_03_Test_01` (`SkeletalMeshComponent.GetAnimInstance` (`self.Mesh`))))
      (bind _custom_location_to_look_at (`self.Custom_Location_To_Look_At`)
        (:`then`
          (set `/Game/Assets/Characters/MainCharacter/6/ABP_Courier_03_Test_01.Player_Camera_Location` (`SceneComponent.K2_GetComponentLocation` _custom_location_to_look_at) _asabp_courier_03_test_01)
          (set `/Game/Assets/Characters/MainCharacter/6/ABP_Courier_03_Test_01.Use_Player_Rotation_Alpha` (`self.PlayerAlpha`) _asabp_courier_03_test_01))
        (:`else`)))))

(event `self.ReceiveTick`
  (params (DeltaSeconds :type "Float (single-precision)"))
  (bind _custom_location_to_look_at (`self.Custom_Location_To_Look_At`)
    (:`then`
      (bind _asabp_courier_03_test_01 (cast `/Game/Assets/Characters/MainCharacter/6/ABP_Courier_03_Test_01` (`SkeletalMeshComponent.GetAnimInstance` (`self.Mesh`))))
      (set `/Game/Assets/Characters/MainCharacter/6/ABP_Courier_03_Test_01.Player_Camera_Location` (`SceneComponent.K2_GetComponentLocation` _custom_location_to_look_at) _asabp_courier_03_test_01)
      (set `/Game/Assets/Characters/MainCharacter/6/ABP_Courier_03_Test_01.Use_Player_Rotation_Alpha` (`self.PlayerAlpha`) _asabp_courier_03_test_01))
    (:`else`)))

(fn `UserConstructionScript`)